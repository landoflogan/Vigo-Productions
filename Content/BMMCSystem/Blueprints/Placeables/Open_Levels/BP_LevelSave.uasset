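; BP_LevelSave is a placeable trigger that records the current level name to a save game when the player character overlaps its box.
; On overlap by BP_MainCharacter, it loads slot SaveGame1, or creates a new OBJ_Save if none exists, sets LevelName and writes the slot back.
; A DoOnce ahead of the character check means the first overlap by any actor uses up the trigger.
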(event OnComponentBeginOverlap(Box)
  (params (OverlappedComponent :type Primitive%20Component%20Object%20Reference) (OtherActor :type Actor%20Object%20Reference) (OtherComp :type Primitive%20Component%20Object%20Reference) (OtherBodyIndex :type Integer) (bFromSweep :type Boolean) (SweepResult :type Hit%20Result%20Structure%20%28by%20ref%29))
  (Utilities|FlowControl|DoOnce false
    (:Completed
      (Utilities|Casting|CastToBP_MainCharacter OtherActor)
      (bind _returnvalue (SaveGame|DoesSaveGameExist "SaveGame1"))
      (if _returnvalue
        (bind _returnvalue_2 (SaveGame|LoadGamefromSlot "SaveGame1"))
        (bind _output_get (Variables|Default|SetSave%20Sub%20Class _returnvalue_2))
        (bind _asobj_save (Utilities|Casting|CastToOBJ_Save _output_get))
        (bind _returnvalue_3 (Game|GetCurrentLevelName true))
        (Variables|/Game/BMMCSystem/Blueprints/Placeables/Save/OBJ_Save.OBJ_Save_C|SetLevel%20Name _asobj_save _returnvalue_3)
        (else
          (bind _returnvalue_4 (SaveGame|CreateSaveGameObject "/Game/BMMCSystem/Blueprints/Placeables/Save/OBJ_Save.OBJ_Save_C"))
          (bind _output_get_2 (Variables|Default|SetSave%20Sub%20Class _returnvalue_4))
          (bind _asobj_save_2 (Utilities|Casting|CastToOBJ_Save _output_get_2))
          (bind _returnvalue_5 (Game|GetCurrentLevelName true))
          (Variables|/Game/BMMCSystem/Blueprints/Placeables/Save/OBJ_Save.OBJ_Save_C|SetLevel%20Name _asobj_save_2 _returnvalue_5)))
      (Development|PrintString "Saving...")
      (SaveGame|SaveGametoSlot (Variables|Default|GetSave%20Sub%20Class) "SaveGame1"))))

(event EventBeginPlay)

(event Collision|EventActorBeginOverlap
  (params (OtherActor :type Actor%20Object%20Reference)))

(event EventTick
  (params (DeltaSeconds :type Float%20%28single-precision%29)))

(fn ConstructionScript)