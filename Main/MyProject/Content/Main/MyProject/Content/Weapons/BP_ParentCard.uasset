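; BP_ParentCard is the base class for cards held in an owner's AC_Magic component.
; It declares an empty Used event that receives a casting transform, apparently for child cards to implement.
; RemoveCardFromHand looks up the card in the owner's AC_Magic Cards array and removes it, printing a debug message if the component or card is missing.
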(event Custom|Remove%20Card%20From%20Hand
  (bind _returnvalue (Components|GetOwner))
  (bind _self self)
  (bind _returnvalue_2 (Actor|GetComponentbyClass _returnvalue "/Game/Weapons/Componets/AC_Magic.AC_Magic_C"))
  (bind _cards (Variables|/Game/Weapons/Componets/AC_Magic.AC_Magic_C|GetCards _returnvalue_2))
  (bind _returnvalue_3 (Utilities|Array|FindItem _cards _self))
  (Utilities|IsValid _returnvalue_2
    (:Is%20Valid
      (if (> _returnvalue_3 -1)
        (Utilities|Array|RemoveIndex _cards _returnvalue_3)
        (else
          (Development|PrintString "Card not found (Card was probally already deleted)"))))
    (:Is%20Not%20Valid
      (Development|PrintString "Owner does not implement AC_Magic (owner should not have card)"))))

(event Custom|Used
  (params (Casting%20Transform :type Transform)))