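; Health component that tracks an actor's hit points and handles its death.
; Health starts at MaxHealth on BeginPlay, and AddDamage subtracts from it.
; At zero or below, a Character owner stops active movement, plays the death montage and is destroyed after a delay equal to the montage's duration.
; Owners that are not Characters fail the cast, so this path never destroys them.
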(event Custom|Add%20Damage
  (params (Damage :type Float%20%28double-precision%29))
  (bind _output_get (Variables|Default|SetHealth (- (Variables|Default|GetHealth) Damage)))
  (if (<= _output_get 0.0)
    (bind _ascharacter (Utilities|Casting|CastToCharacter (Components|GetOwner)))
    (Class|NavMovementComponent|StopActiveMovement (Variables|/Script/Engine.Character|GetCharacterMovement _ascharacter))
    (bind _returnvalue (Animation|Montage|MontagePlay (Components|SkeletalMesh|GetAnimInstance (Variables|/Script/Engine.Character|GetMesh _ascharacter)) "/Game/AI/imports/M_Death.M_Death" 1.0 "Duration" 0.0 true))
    (Utilities|FlowControl|Delay _returnvalue)
    (CallFunction|Die)))

(event Custom|Die
  (Actor|DestroyActor (Components|GetOwner self)))

(event EventBeginPlay
  (Variables|Default|SetHealth (Variables|Default|GetMax%20Health)))