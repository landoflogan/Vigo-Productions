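; BP_Bullet is a projectile weapon bullet that damages whatever it hits.
; On BeginPlay it adds the velocity of player character 0 to its ProjectileMovement velocity, so shots inherit that character's motion.
; Impacts are handled through the projectile bounce event, which passes Damage to the hit actor's AC_Health component, or prints a debug string if none exists.
; The bullet destroys itself after that first bounce.
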(event OnProjectileBounce(ProjectileMovement)
  (params (ImpactResult :type Hit%20Result%20Structure%20%28by%20ref%29) (ImpactVelocity :type Vector%20%28by%20ref%29 :default "0, 0, 0"))
  (bind _returnvalue (Actor|GetComponentbyClass (.hitactor ImpactResult) "/Game/Weapons/Componets/AC_Health.AC_Health_C"))
  (Utilities|IsValid _returnvalue
    (:Is%20Valid
      (Default|AddDamage _returnvalue (Variables|Default|GetDamage)))
    (:Is%20Not%20Valid
      (Development|PrintString "Hello")))
  (Actor|DestroyActor))

(event EventBeginPlay
  (bind _projectilemovement (Variables|Default|GetProjectileMovement))
  (Variables|/Script/Engine.MovementComponent|SetVelocity _projectilemovement (+ (Transformation|GetVelocity (Game|GetPlayerCharacter 0)) (Variables|/Script/Engine.MovementComponent|GetVelocity _projectilemovement))))

(fn ConstructionScript)