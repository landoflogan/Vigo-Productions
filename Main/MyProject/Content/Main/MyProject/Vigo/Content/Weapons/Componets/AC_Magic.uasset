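; AC_Magic is a component that manages a set of magic cards on its owner, one active at a time.
; SetupMagic spawns each card class as a component on the owner, attaches it to the skeleton at that card's socket, then selects the first.
; SwitchCard hides all but the chosen card and makes it active, and UseCard passes the shooting transform to it.
; Comments flag setup and switching for possible rework.
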(event Custom|Use%20Card
  (params (Shooting%20Transform :type Transform))
  ;[1 1 1] Card Using
  (Default|Used (Variables|Default|GetActiveCard) Shooting%20Transform))

(event Custom|Switch%20Card
  (params (NewWeaponNum :type Integer))
  ;[1 0.9077 0] Card Switching (Needs to be Redone)
  (for (_array_element _array_index) (Variables|Default|GetCards)
    (Development|SetHiddeninGame _array_element (!= _array_index NewWeaponNum) false)
    (if (not (!= _array_index NewWeaponNum))
      (Variables|Default|SetActiveCard (Utilities|Array|Get(acopy) (Variables|Default|GetCards) NewWeaponNum))
      (Variables|Default|SetCardIndex NewWeaponNum))))

(event Custom|Setup%20Magic
  (params (Skeleton :type Scene%20Component%20Object%20Reference) (Weapons%20Array :type Array%20of%20Skeletal%20Mesh%20Component%20Class%20References))
  ;[1 0.9027 0] Magic Setup (Might need to be redone)
  (for _array_element Weapons%20Array
    (Utilities|Array|Add (Variables|Default|GetCards) 0))
  (for (_ _array_index) (Variables|Default|GetCards)
    (bind _returnvalue (Game|AddComponentbyClass (Components|GetOwner) (Utilities|Array|Get(acopy) Weapons%20Array _array_index) false))
    (bind _asbp_parent_card (Utilities|Casting|CastToBP_ParentCard _returnvalue)
      (:then
        (Utilities|Array|SetArrayElem (Variables|Default|GetCards) _array_index _asbp_parent_card)
        (Transformation|AttachComponentToComponent _returnvalue Skeleton (Variables|/Game/Weapons/BP_ParentCard.BP_ParentCard_C|GetSocket _asbp_parent_card) "KeepRelative" "KeepRelative" "KeepRelative" true))
      (:CastFailed
        (Development|PrintString "Cast Failed (not card)"))))
  (CallFunction|SwitchCard))